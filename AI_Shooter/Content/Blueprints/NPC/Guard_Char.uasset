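; Guard NPC character that spawns with a weapon in its hand socket and exposes combat, patrol and state hooks for AI control.
; State and aiming changes are forwarded to the AnimInstance by message, while walk speed follows the guard's state.
; Fire requests and range queries pass through to the weapon.
; HealthComponent events play a hit-react montage on damage and, once on death, ragdoll the mesh and stop the AI brain.
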(event OnDamageTaken(HealthComponent)
  (Animation|PlayAnimMontage "/Game/Characters/Animations/Hit_React_1_Montage.Hit_React_1_Montage" 1.0 "None"))

(event OnDeath(HealthComponent)
  ;[1 1 1] Rip check
  (Utilities|FlowControl|DoOnce false
    (:Completed
      (Collision|SetCollisionProfileName (Variables|Character|GetMesh) "Ragdoll" true :!class /Script/Engine.PrimitiveComponent)
      (Class|SkeletalMeshComponent|SetAllBodiesSimulatePhysics (Variables|Character|GetMesh) true)
      (Class|PrimitiveComponent|WakeAllRigidBodies (Variables|Character|GetMesh))
      (Collision|SetCollisionEnabled (Variables|Collision|GetCapsuleComponent) "NoCollision")
      (Development|PrintString (Utilities|String|Append (Utilities|GetDisplayName self) " Died!"))
      (AI|Logic|StopLogic (Variables|/Script/AIModule.AIController|GetBrainComponent (AI|GetAIController 0)) (Variables|Default|GetReason)))))

(event Custom|CustomEvent
  (params (IsAiming :type Boolean)))

(event EventBeginPlay
  (bind _self self)
  ;[1 1 1] Giving Weapon
  (bind _returnvalue (Game|SpawnActorfromClass (Variables|Default|GetWeaponClass) (CallFunction|IdentityTransform) "AlwaysSpawn" "SelectDefaultAtRuntime" _self _self))
  (bind _output_get (Variables|Default|SetWeapon _returnvalue))
  (Transformation|AttachComponentToComponent _output_get (Variables|Character|GetMesh) "WeaponSocket" "SnapToTarget" "SnapToTarget" "SnapToTarget" true))

(event Collision|EventActorBeginOverlap
  (params (OtherActor :type Actor%20Object%20Reference)))

(event EventTick
  (params (DeltaSeconds :type Float%20%28single-precision%29)))

(event EventNotifyStateChanged
  (params (NewState :type NPC_State%20Enum :default "NewEnumerator0"))
  ;[1 1 1] On State Changed
  (Class|BPIAIHelper|NotifyStateChanged(Message) (Components|SkeletalMesh|GetAnimInstance (Variables|Character|GetMesh)) NewState))

(event EventModifyMovementSpeed
  (params (State :type NPC_State%20Enum :default "NewEnumerator0"))
  ;[1 1 1] Setting movement speed
  (Variables|/Script/Engine.CharacterMovementComponent|SetMaxWalkSpeed (Variables|Character|GetCharacterMovement) (Utilities|Select :Index State :NewEnumerator0 1.6e+02 :NewEnumerator1 1.6e+02 :NewEnumerator2 4e+02 :NewEnumerator3 6e+02 :NewEnumerator4 0.0)))

(event EventModifyAimingStance
  (params (IsAiming :type Boolean))
  ;[1 1 1] Is Aiming
  (Class|BPIAIHelper|ModifyAimingStance(Message) (Components|SkeletalMesh|GetAnimInstance (Variables|Character|GetMesh)) IsAiming))

(event EventTryShootEquippedWeapon
  ;[1 1 1] Try Sgoot Gun via Interface
  (bind _weapon (Variables|Default|GetWeapon)
    (:then
      (Default|OnFireRequested _weapon))
    (:else)))

(fn ConstructionScript)

(fn GetIsDead
  (return (Default|IsDead (Variables|Default|GetHealthComponent))))

(fn GetPatrolRoute
  (return (Variables|Default|GetMyPatrolPath)))

(fn GetTeamID
  (return false))

(fn GetWeapon
  (bind _weapon (Variables|Default|GetWeapon))
  (return (Utilities|IsValid _weapon) _weapon))

(fn GetWeaponRange
  (return (Variables|/Game/Blueprints/Weapons/WeaponBase.WeaponBase_C|GetWeaponRange (Variables|Default|GetWeapon))))